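; Starting room Blueprint where up to four players ready up through exit boxes and the next dungeon room can be spawned.
; Each one-shot box overlap hides, disables and nudges the player, increments NBPlayerReady and triggers a door timeline.
; All four timelines move DoorPlayerExit4, each lerping upward from a different door's location.
; FNextRoom, not called here, spawns a grid-snapped room from BP_GestionGame's layout table, trace-checking the larger type.
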(event `C_RoomEnter`
  (params (Index :type Integer))
  (bind _returnvalue (`SceneComponent.K2_GetComponentLocation` (`self.DoorPlayerExit4`)))
  (bind _returnvalue_2 (`SceneComponent.K2_GetComponentLocation` (`self.DoorPlayerExit1`)))
  (bind _returnvalue_3 (`SceneComponent.K2_GetComponentLocation` (`self.DoorPlayerExit2`)))
  (bind _returnvalue_4 (`SceneComponent.K2_GetComponentLocation` (`self.DoorPlayerExit3`)))
  (switch `int` Index
    (:`0`
      (bind (_direction _time) (`Timeline|T_Doors` :!via `PlayFromStart`)
        (:`Update`
          (`SceneComponent.K2_SetWorldLocation` (`self.DoorPlayerExit4`) (`KismetMathLibrary.VLerp` _returnvalue_2 (+ _returnvalue_2 (0.0 0.0 250.0)) _time) false false))))
    (:`1`
      (bind (_direction_2 _time_2) (`Timeline|Timeline` :!via `PlayFromStart`)
        (:`Update`
          (`SceneComponent.K2_SetWorldLocation` (`self.DoorPlayerExit4`) (`KismetMathLibrary.VLerp` _returnvalue_3 (+ _returnvalue_3 (0.0 0.0 250.0)) _time_2) false false))))
    (:`2`
      (bind (_direction_3 _time_3) (`Timeline|Timeline_0` :!via `PlayFromStart`)
        (:`Update`
          (`SceneComponent.K2_SetWorldLocation` (`self.DoorPlayerExit4`) (`KismetMathLibrary.VLerp` _returnvalue_4 (+ _returnvalue_4 (0.0 0.0 250.0)) _time_3) false false))))
    (:`3`
      (bind (_direction_4 _time_4) (`Timeline|Timeline_1` :!via `PlayFromStart`)
        (:`Update`
          (`SceneComponent.K2_SetWorldLocation` (`self.DoorPlayerExit4`) (`KismetMathLibrary.VLerp` _returnvalue (+ _returnvalue (0.0 0.0 15.0)) _time_4) false false))))))

(event `self.Box1.OnComponentBeginOverlap`
  (params (OverlappedComponent :type "PrimitiveComponent Object Reference") (OtherActor :type "Actor Object Reference") (OtherComp :type "PrimitiveComponent Object Reference") (OtherBodyIndex :type Integer) (bFromSweep :type Boolean) (SweepResult :type "HitResult Structure (by ref)"))
  (`/Engine/EditorBlueprintResources/StandardMacros.DoOnce` false
    (:`Completed`
      (bind _asbp_player (cast `/Game/BP/Players/BP_Player` OtherActor))
      (bind _aspc_player (cast `/Game/BP/Players/PC_Player` (`Pawn.GetController` _asbp_player)))
      (`self.SetActorHiddenInGame` _asbp_player true)
      (`self.DisableInput` _asbp_player _aspc_player)
      (`self.K2_SetActorLocation` _asbp_player (+ (`self.K2_GetActorLocation` _asbp_player) (100.0 0.0 0.0)) false false)
      (`/Engine/EditorBlueprintResources/StandardMacros.IncrementInt` (`self.NBPlayerReady`)
        (:`  `
          (`self.C_RoomEnter` 0))))))

(event `self.Box2.OnComponentBeginOverlap`
  (params (OverlappedComponent :type "PrimitiveComponent Object Reference") (OtherActor :type "Actor Object Reference") (OtherComp :type "PrimitiveComponent Object Reference") (OtherBodyIndex :type Integer) (bFromSweep :type Boolean) (SweepResult :type "HitResult Structure (by ref)"))
  (`/Engine/EditorBlueprintResources/StandardMacros.DoOnce` false
    (:`Completed`
      (bind _asbp_player (cast `/Game/BP/Players/BP_Player` OtherActor))
      (bind _aspc_player (cast `/Game/BP/Players/PC_Player` (`Pawn.GetController` _asbp_player)))
      (`self.SetActorHiddenInGame` _asbp_player true)
      (`self.DisableInput` _asbp_player _aspc_player)
      (`self.K2_SetActorLocation` _asbp_player (+ (`self.K2_GetActorLocation` _asbp_player) (100.0 0.0 0.0)) false false)
      (`/Engine/EditorBlueprintResources/StandardMacros.IncrementInt` (`self.NBPlayerReady`)
        (:`  `
          (`self.C_RoomEnter` 1))))))

(event `self.Box3.OnComponentBeginOverlap`
  (params (OverlappedComponent :type "PrimitiveComponent Object Reference") (OtherActor :type "Actor Object Reference") (OtherComp :type "PrimitiveComponent Object Reference") (OtherBodyIndex :type Integer) (bFromSweep :type Boolean) (SweepResult :type "HitResult Structure (by ref)"))
  (`/Engine/EditorBlueprintResources/StandardMacros.DoOnce` false
    (:`Completed`
      (bind _asbp_player (cast `/Game/BP/Players/BP_Player` OtherActor))
      (bind _aspc_player (cast `/Game/BP/Players/PC_Player` (`Pawn.GetController` _asbp_player)))
      (`self.SetActorHiddenInGame` _asbp_player true)
      (`self.DisableInput` _asbp_player _aspc_player)
      (`self.K2_SetActorLocation` _asbp_player (+ (`self.K2_GetActorLocation` _asbp_player) (100.0 0.0 0.0)) false false)
      (`/Engine/EditorBlueprintResources/StandardMacros.IncrementInt` (`self.NBPlayerReady`)
        (:`  `
          (`self.C_RoomEnter` 2))))))

(event `self.Box4.OnComponentBeginOverlap`
  (params (OverlappedComponent :type "PrimitiveComponent Object Reference") (OtherActor :type "Actor Object Reference") (OtherComp :type "PrimitiveComponent Object Reference") (OtherBodyIndex :type Integer) (bFromSweep :type Boolean) (SweepResult :type "HitResult Structure (by ref)"))
  (`/Engine/EditorBlueprintResources/StandardMacros.DoOnce` false
    (:`Completed`
      (bind _asbp_player (cast `/Game/BP/Players/BP_Player` OtherActor))
      (bind _aspc_player (cast `/Game/BP/Players/PC_Player` (`Pawn.GetController` _asbp_player)))
      (`self.SetActorHiddenInGame` _asbp_player true)
      (`self.DisableInput` _asbp_player _aspc_player)
      (`self.K2_SetActorLocation` _asbp_player (+ (`self.K2_GetActorLocation` _asbp_player) (100.0 0.0 0.0)) false false)
      (`/Engine/EditorBlueprintResources/StandardMacros.IncrementInt` (`self.NBPlayerReady`)
        (:`  `
          (`self.C_RoomEnter` 3))))))

(fn `F_NextRoom`
  (bind _returnvalue (+ (`self.K2_GetActorLocation`) (1500.0 -2250.0 0.0)))
  (bind _returnvalue_2 (`GameplayStatics.GetActorOfClass` "/Game/BP/GenereteDonjon/BP_GestionGame.BP_GestionGame_C"))
  (switch `int` (`self.RoomIndex`)
    (:`0`
      (bind _x (`KismetMathLibrary.BreakVector4` (`|GetArrayItem` (`/Game/BP/GenereteDonjon/BP_GestionGame.TableDonjonCreate` _returnvalue_2) (+ (`self.NBRoom`) 1))))
      (if (== _x 1.0)
        (`|SpawnActorFromClass` "/Game/BP/Room/RoomBasic/BP_RoomDefault.BP_RoomDefault_C" (`KismetMathLibrary.MakeTransform` (`KismetMathLibrary.Vector_SnappedToGrid` (+ (`self.K2_GetActorLocation`) (1500.0 0.0 0.0)) 1500.0)) "Undefined" "MultiplyWithRoot" null 0 null)
        (elif (== _x 2.0)
          (bind (_outhit _returnvalue_3) (`KismetSystemLibrary.SphereTraceSingleForObjects` _returnvalue _returnvalue 20.0 (`|MakeArray` "ObjectTypeQuery7" :!type "EObjectTypeQuery Enum")))
          (if _returnvalue_3
            (return)
            (else
              (`|SpawnActorFromClass` "/Game/BP/Room/Room2P/BP_2RoomDefault.BP_2RoomDefault_C" (`KismetMathLibrary.MakeTransform` (`KismetMathLibrary.Vector_SnappedToGrid` (+ (`self.K2_GetActorLocation`) (1500.0 -2250.0 0.0)) 1500.0)) "Undefined" "MultiplyWithRoot" null 0 null)))
          (elif (== _x 4.0)
            _))))))

(fn `UserConstructionScript`)