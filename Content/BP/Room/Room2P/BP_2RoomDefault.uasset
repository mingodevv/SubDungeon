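; BP_2RoomDefault is a combat room that locks the player in, runs a monster fight, then chains to the next room.
; Player overlap triggers a one-shot timeline sliding both doors, then spawns up to four melee monsters with poof effects.
; Death events spawn replacements until the quota is met, then spawn BP_RoomDefault on a snapped grid and reverse the exit door.
; It also randomizes two planes' material colors and offers a one-shot camera blend.
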(event `self.ReceiveBeginPlay`
  (bind _returnvalue (`KismetMathLibrary.RandomFloatInRange` 0.0 1.0))
  (bind _returnvalue_2 (`KismetMathLibrary.RandomFloatInRange` 0.0 1.0))
  (bind _returnvalue_3 (`KismetMathLibrary.RandomFloatInRange` 0.0 1.0))
  (bind _returnvalue_4 (`PrimitiveComponent.CreateDynamicMaterialInstance` (`self.Plane1`) 0 "/Game/Material/Basic/M_Random.M_Random" "None"))
  (bind _returnvalue_5 (`PrimitiveComponent.CreateDynamicMaterialInstance` (`self.Plane2`) 0 "/Game/Material/Basic/M_Random.M_Random" "None"))
  (`MaterialInstanceDynamic.SetVectorParameterValue` _returnvalue_4 "test" (make `LinearColor` _returnvalue_2 _returnvalue_3 _returnvalue 1.0))
  (`MaterialInstanceDynamic.SetVectorParameterValue` _returnvalue_5 "test" (make `LinearColor` _returnvalue_2 _returnvalue_3 0.0 _returnvalue)))

(event `self.PlayerPlace.OnComponentBeginOverlap`
  (params (OverlappedComponent :type "PrimitiveComponent Object Reference") (OtherActor :type "Actor Object Reference") (OtherComp :type "PrimitiveComponent Object Reference") (OtherBodyIndex :type Integer) (bFromSweep :type Boolean) (SweepResult :type "HitResult Structure (by ref)"))
  (cast `/Game/BP/Players/BP_Player` OtherActor)
  (`/Engine/EditorBlueprintResources/StandardMacros.DoOnce` false
    (:`Completed`
      (`self.C_RoomEnter`))))

(event `C_TargetCam`
  (params (PlayerController :type "/Game/BP/Players/PC_Player Object Reference"))
  (`/Engine/EditorBlueprintResources/StandardMacros.DoOnce` false
    (:`Completed`
      (`PlayerController.SetViewTargetWithBlend` PlayerController (`ChildActorComponent.ChildActor` (`self.Camera`)) 0.5 "VTBlend_Linear" 0.0 false))))

(event `C_RoomEnter`
  (set `self.LocExitDoors` (`SceneComponent.K2_GetComponentLocation` (`self.DoorPlayerExit`)))
  (set `self.LocEnterDoors` (`SceneComponent.K2_GetComponentLocation` (`self.DoorPlayerenter`)))
  (bind (_direction _time) (`Timeline|T_Doors` :!via `PlayFromStart`)
    (:`Update`
      (`SceneComponent.K2_SetWorldLocation` (`self.DoorPlayerExit`) (`KismetMathLibrary.VLerp` (`self.LocExitDoors`) (`SceneComponent.K2_GetComponentLocation` (`self.BExit`)) _time) false false)
      (`SceneComponent.K2_SetWorldLocation` (`self.DoorPlayerenter`) (`KismetMathLibrary.VLerp` (`self.LocEnterDoors`) (`SceneComponent.K2_GetComponentLocation` (`self.BEnter`)) _time) false false))
    (:`Finished`
      (`self.C_SpawnMonster`))))

(event `C_MonsterDead`
  (params (Int :type Integer))
  (bind _output_get (set `self.NBMonsterDead` (+ Int (`self.NBMonsterDead`))))
  (if (== (`self.NBMonsterMax`) _output_get)
    (`|SpawnActorFromClass` "/Game/BP/Room/RoomBasic/BP_RoomDefault.BP_RoomDefault_C" (`KismetMathLibrary.MakeTransform` (`KismetMathLibrary.Vector_SnappedToGrid` (+ (`self.K2_GetActorLocation`) (1500.0 0.0 0.0)) 1500.0)) "Undefined" "MultiplyWithRoot" null 0 null)
    (bind (_direction _time) (`Timeline|T_DoorsExit` :!via `ReverseFromEnd`)
      (:`Update`
        (`SceneComponent.K2_SetWorldLocation` (`self.DoorPlayerExit`) (`KismetMathLibrary.VLerp` (`self.LocExitDoors`) (`SceneComponent.K2_GetComponentLocation` (`self.BExit`)) _time) false false)))
    (elif (not (== (`self.NBMonsterActualy`) (`self.NBMonsterMax`)))
      (bind _output_get_2 (set `self.RandomPoint` (`KismetArrayLibrary.Array_Random` (`|MakeArray` (`self.Spawn1`) (`self.Spawn4`) (`self.Spawn3`) (`self.Spawn2`)))))
      (bind (_returnvalue_location _returnvalue_rotation) (`KismetMathLibrary.BreakTransform` (`SceneComponent.K2_GetComponentToWorld` _output_get_2)))
      (`NiagaraFunctionLibrary.SpawnSystemAtLocation` "/Game/Particule/Poof/N_Poof.N_Poof" _returnvalue_location)
      (`AIBlueprintHelperLibrary.SpawnAIFromClass` "/Game/BP/Monster/Test/BP_MonsterCACDefault.BP_MonsterCACDefault_C" null _returnvalue_location _returnvalue_rotation false null)
      (`/Engine/EditorBlueprintResources/StandardMacros.IncrementInt` (`self.NBMonsterActualy`)))))

(event `C_SpawnMonster`
  (bind _output_get (set `self.NBMonsterMax` 5))
  (if (> _output_get 4)
    (set `self.Last Index` 4)
    (else
      (set `self.Last Index` _output_get)))
  (for _index (range 1 (+ (`self.Last Index`) 1))
    (set `self.NBMonsterActualy` _index)
    (bind (_returnvalue_location _returnvalue_rotation) (`KismetMathLibrary.BreakTransform` (`SceneComponent.K2_GetComponentToWorld` (`|GetArrayItem` (`|MakeArray` (`self.Spawn1`) (`self.Spawn4`) (`self.Spawn3`) (`self.Spawn2`)) (- _index 1)))))
    (bind _returnvalue (+ _returnvalue_location (0.0 0.0 30.0)))
    (`NiagaraFunctionLibrary.SpawnSystemAtLocation` "/Game/Particule/Poof/N_Poof.N_Poof" _returnvalue)
    (`AIBlueprintHelperLibrary.SpawnAIFromClass` "/Game/BP/Monster/Test/BP_MonsterCACDefault.BP_MonsterCACDefault_C" null _returnvalue _returnvalue_rotation false null)))

(fn `UserConstructionScript`)