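; Default melee monster that chases any pawn it sees and damages players it reaches.
; On BeginPlay a line trace from A to B finds and stores the BP_RoomDefault it stands in.
; PawnSensing drives AIMoveTo; on arrival, an A-to-C trace sends damage through BPI_Players to the hit actor.
; FMonsterDammage destroys the monster on its first call, with no health check, after reporting the death to the stored room.
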(event `self.ReceiveBeginPlay`
  (`self.F_LineFoot`))

(event `self.PawnSensing.OnSeePawn`
  (params (Pawn :type "Pawn Object Reference"))
  (`/Engine/EditorBlueprintResources/StandardMacros.IsValid` Pawn
    (:`Is Valid`
      (`|AIMoveTo` self (0.0 0.0 0.0) Pawn
        (:`OnSuccess`
          (bind (_outhit _returnvalue) (`KismetSystemLibrary.LineTraceSingleForObjects` (`SceneComponent.K2_GetComponentLocation` (`self.A`)) (`SceneComponent.K2_GetComponentLocation` (`self.C`)) (`|MakeArray` "ObjectTypeQuery9" :!type "EObjectTypeQuery Enum")))
          (if _returnvalue
            (bind (_bblockinghit _binitialoverlap _time _distance _location _impactpoint _normal _impactnormal _physmat _hitactor) (`GameplayStatics.BreakHitResult` _outhit))
            (if (`KismetSystemLibrary.DoesImplementInterface` _hitactor "/Game/BP/Players/BPI_Players.BPI_Players_C")
              (message `/Game/BP/Players/BPI_Players.F_DamagePlayers` _hitactor (`self.Damage`)))))))))

(event `/Game/BP/Monster/BPI_Monster.F_MonsterDammage`
  (params (Damage :type "Float (double-precision)"))
  (bind _asbp_room_default (cast `/Game/BP/Room/RoomBasic/BP_RoomDefault` (`self.RefRoomMonster`)))
  (`/Game/BP/Room/RoomBasic/BP_RoomDefault.C_MonsterDead` _asbp_room_default 1)
  (`self.K2_DestroyActor`))

(fn `F_LineFoot`
  (bind (_outhit _returnvalue) (`KismetSystemLibrary.LineTraceSingleForObjects` :`Start` (`SceneComponent.K2_GetComponentLocation` (`self.A`)) :`End` (`SceneComponent.K2_GetComponentLocation` (`self.B`)) :`ObjectTypes` (`|MakeArray` "ObjectTypeQuery7" :!type "EObjectTypeQuery Enum") :`DrawDebugType` "ForOneFrame"))
  (if _returnvalue
    (bind _asbp_room_default (cast `/Game/BP/Room/RoomBasic/BP_RoomDefault` (`.HitActor` (`GameplayStatics.BreakHitResult` _outhit))))
    (set `self.RefRoomMonster` _asbp_room_default)))

(fn `UserConstructionScript`)