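; Dungeon generator actor that lays out a procedural 100-step dungeon of four-lane room rows at BeginPlay.
; It spawns a start room, and for multiplayer M2RoomInsert shuffles random two-player slots into Map2Room.
; Each step becomes a Vector4 lane-width code: boss indices span all four lanes, others mix two-wide and single rooms.
; A second pass spawns random room classes from size-matched arrays, grid-snapped along X.
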(event `self.ReceiveBeginPlay`
  (bind _returnvalue (`self.GetTransform`))
  (bind _asgi_sub_donjon (cast `/Game/BP/Players/GI_SubDonjon` (`GameplayStatics.GetGameInstance`)))
  (switch `int` (`/Game/BP/Players/GI_SubDonjon.NBPlayer` _asgi_sub_donjon)
    (:`1`
      (`|SpawnActorFromClass` "/Game/BP/Room/RoomBegin/BP_BRoomDefault1.BP_BRoomDefault1_C" _returnvalue "Undefined" "MultiplyWithRoot" null -1 null))
    (:`2`
      (`|SpawnActorFromClass` "/Game/BP/Room/RoomBegin/BP_BRoomDefault1.BP_BRoomDefault1_C" _returnvalue "Undefined" "MultiplyWithRoot" null -1 null)
      (`self.M_2RoomInsert` :!label _label
        (:`completed`
          _)))
    (:`3`
      (`|SpawnActorFromClass` "/Game/BP/Room/RoomBegin/BP_BRoomDefault1.BP_BRoomDefault1_C" _returnvalue "Undefined" "MultiplyWithRoot" null -1 null)
      (goto _label))
    (:`4`
      (`|SpawnActorFromClass` "/Game/BP/Room/RoomBegin/BP_BRoomDefault1.BP_BRoomDefault1_C" _returnvalue "Undefined" "MultiplyWithRoot" null -1 null)
      (goto _label)))
  (for _index (range 100)
    (if (!= (`KismetArrayLibrary.Array_Find` (`self.ArrayBossIndex`) _index) -1)
      (`KismetArrayLibrary.Array_Add` (`self.TableDonjonCreate`) (`KismetMathLibrary.MakeVector4` 4.0 4.0 4.0 4.0))
      (elif (`|GetArrayItem` (`self.Map2Room`) _index)
        (bind _output_get (set `self.IntRandomFor2Room` (`KismetMathLibrary.RandomInteger` 2)))
        (switch `int` _output_get
          (:`0`
            (`KismetArrayLibrary.Array_Add` (`self.TableDonjonCreate`) (`KismetMathLibrary.MakeVector4` 2.0 2.0 1.0 1.0)))
          (:`1`
            (`KismetArrayLibrary.Array_Add` (`self.TableDonjonCreate`) (`KismetMathLibrary.MakeVector4` 1.0 2.0 2.0 1.0)))
          (:`2`
            (`KismetArrayLibrary.Array_Add` (`self.TableDonjonCreate`) (`KismetMathLibrary.MakeVector4` 1.0 1.0 2.0 2.0))))
        (else
          (`KismetArrayLibrary.Array_Add` (`self.TableDonjonCreate`) (`KismetMathLibrary.MakeVector4` 1.0 1.0 1.0 1.0))))))
  (for (_array_element _array_index) (`self.TableDonjonCreate`)
    (set `self.NBRoom` _array_index)
    (set `self.NBLastX` (+ (`self.NBLastX`) 1500))
    (bind (_x _y _z) (`KismetMathLibrary.BreakVector4` _array_element))
    (if (== _x 4.0)
      (`|SpawnActorFromClass` (`KismetArrayLibrary.Array_Random` (`self.ArrayRoom4P`)) (`KismetMathLibrary.MakeTransform` (`KismetMathLibrary.Vector_SnappedToGrid` (`KismetMathLibrary.MakeVector` (`KismetMathLibrary.Conv_IntToDouble` (`self.NBLastX`))) 750.0)) "Undefined" "MultiplyWithRoot" null null)
      (set `self.NBLastX` (+ (`self.NBLastX`) 3000))
      (elif (== _x 2.0)
        (`|SpawnActorFromClass` (`KismetArrayLibrary.Array_Random` (`self.ArrayRoom2P`)) (`KismetMathLibrary.MakeTransform` (`KismetMathLibrary.Vector_SnappedToGrid` (`KismetMathLibrary.MakeVector` (`KismetMathLibrary.Conv_IntToDouble` (`self.NBLastX`)) -1500.0) 750.0)) "Undefined" "MultiplyWithRoot" null null)
        (`|SpawnActorFromClass` (`KismetArrayLibrary.Array_Random` (`self.ArrayRoom1P`)) (`KismetMathLibrary.MakeTransform` (`KismetMathLibrary.Vector_SnappedToGrid` (`KismetMathLibrary.MakeVector` (`KismetMathLibrary.Conv_IntToDouble` (`self.NBLastX`)) 750.0) 750.0)) "Undefined" "MultiplyWithRoot" null null)
        (`|SpawnActorFromClass` (`KismetArrayLibrary.Array_Random` (`self.ArrayRoom1P`)) (`KismetMathLibrary.MakeTransform` (`KismetMathLibrary.Vector_SnappedToGrid` (`KismetMathLibrary.MakeVector` (`KismetMathLibrary.Conv_IntToDouble` (`self.NBLastX`)) 2250.0) 750.0)) "Undefined" "MultiplyWithRoot" null null)
        (elif (== _y 2.0)
          (`|SpawnActorFromClass` (`KismetArrayLibrary.Array_Random` (`self.ArrayRoom2P`)) (`KismetMathLibrary.MakeTransform` (`KismetMathLibrary.Vector_SnappedToGrid` (`KismetMathLibrary.MakeVector` (`KismetMathLibrary.Conv_IntToDouble` (`self.NBLastX`))) 750.0)) "Undefined" "MultiplyWithRoot" null null)
          (`|SpawnActorFromClass` (`KismetArrayLibrary.Array_Random` (`self.ArrayRoom1P`)) (`KismetMathLibrary.MakeTransform` (`KismetMathLibrary.Vector_SnappedToGrid` (`KismetMathLibrary.MakeVector` (`KismetMathLibrary.Conv_IntToDouble` (`self.NBLastX`)) -2250.0) 750.0)) "Undefined" "MultiplyWithRoot" null null)
          (`|SpawnActorFromClass` (`KismetArrayLibrary.Array_Random` (`self.ArrayRoom1P`)) (`KismetMathLibrary.MakeTransform` (`KismetMathLibrary.Vector_SnappedToGrid` (`KismetMathLibrary.MakeVector` (`KismetMathLibrary.Conv_IntToDouble` (`self.NBLastX`)) 2250.0) 750.0)) "Undefined" "MultiplyWithRoot" null null)
          (elif (== _z 2.0)
            (`|SpawnActorFromClass` (`KismetArrayLibrary.Array_Random` (`self.ArrayRoom2P`)) (`KismetMathLibrary.MakeTransform` (`KismetMathLibrary.Vector_SnappedToGrid` (`KismetMathLibrary.MakeVector` (`KismetMathLibrary.Conv_IntToDouble` (`self.NBLastX`)) 1500.0) 750.0)) "Undefined" "MultiplyWithRoot" null null)
            (`|SpawnActorFromClass` (`KismetArrayLibrary.Array_Random` (`self.ArrayRoom1P`)) (`KismetMathLibrary.MakeTransform` (`KismetMathLibrary.Vector_SnappedToGrid` (`KismetMathLibrary.MakeVector` (`KismetMathLibrary.Conv_IntToDouble` (`self.NBLastX`)) -2250.0) 750.0)) "Undefined" "MultiplyWithRoot" null null)
            (`|SpawnActorFromClass` (`KismetArrayLibrary.Array_Random` (`self.ArrayRoom1P`)) (`KismetMathLibrary.MakeTransform` (`KismetMathLibrary.Vector_SnappedToGrid` (`KismetMathLibrary.MakeVector` (`KismetMathLibrary.Conv_IntToDouble` (`self.NBLastX`)) -750.0) 750.0)) "Undefined" "MultiplyWithRoot" null null)
            (else
              (`|SpawnActorFromClass` (`KismetArrayLibrary.Array_Random` (`self.ArrayRoom1P`)) (`KismetMathLibrary.MakeTransform` (`KismetMathLibrary.Vector_SnappedToGrid` (`KismetMathLibrary.MakeVector` (`KismetMathLibrary.Conv_IntToDouble` (`self.NBLastX`)) -2250.0) 750.0)) "Undefined" "MultiplyWithRoot" null null)
              (`|SpawnActorFromClass` (`KismetArrayLibrary.Array_Random` (`self.ArrayRoom1P`)) (`KismetMathLibrary.MakeTransform` (`KismetMathLibrary.Vector_SnappedToGrid` (`KismetMathLibrary.MakeVector` (`KismetMathLibrary.Conv_IntToDouble` (`self.NBLastX`)) -750.0) 750.0)) "Undefined" "MultiplyWithRoot" null null)
              (`|SpawnActorFromClass` (`KismetArrayLibrary.Array_Random` (`self.ArrayRoom1P`)) (`KismetMathLibrary.MakeTransform` (`KismetMathLibrary.Vector_SnappedToGrid` (`KismetMathLibrary.MakeVector` (`KismetMathLibrary.Conv_IntToDouble` (`self.NBLastX`)) 750.0) 750.0)) "Undefined" "MultiplyWithRoot" null null)
              (`|SpawnActorFromClass` (`KismetArrayLibrary.Array_Random` (`self.ArrayRoom1P`)) (`KismetMathLibrary.MakeTransform` (`KismetMathLibrary.Vector_SnappedToGrid` (`KismetMathLibrary.MakeVector` (`KismetMathLibrary.Conv_IntToDouble` (`self.NBLastX`)) 2250.0) 750.0)) "Undefined" "MultiplyWithRoot" null null))))))))

(fn `UserConstructionScript`)