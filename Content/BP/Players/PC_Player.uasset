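; PC_Player is a player controller that tracks the player's current dungeon room and re-enables input on the player Blueprint.
; On BeginPlay it stores the BP_BRoomDefault4 actor found in the level as the current room.
; C_VisibilityDungeon hides the stored room if valid, then after a short delay stores the passed room, without changing that room's visibility.
; C_InputEnable enables input on the given player for this controller.
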(event `C_InputEnable`
  (params (Bp_Player :type "/Game/BP/Players/BP_Player Object Reference"))
  (`self.EnableInput` Bp_Player self))

(event `self.ReceiveBeginPlay`
  (bind _returnvalue (`GameplayStatics.GetActorOfClass` "/Game/BP/Room/RoomBegin/BP_BRoomDefault4.BP_BRoomDefault4_C"))
  (set `self.ActorRoomRef` _returnvalue))

(event `C_VisibilityDungeon`
  (params (NewRoom :type "Actor Object Reference"))
  (bind _actorroomref (`self.ActorRoomRef`))
  (`/Engine/EditorBlueprintResources/StandardMacros.IsValid` _actorroomref
    (:`Is Valid`
      (`self.SetActorHiddenInGame` _actorroomref true))
    (:`Is Not Valid`
      _))
  (`KismetSystemLibrary.Delay` 0.2)
  (set `self.ActorRoomRef` NewRoom))

(fn `UserConstructionScript`)